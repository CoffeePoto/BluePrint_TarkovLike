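; BP_Gun is a gun Blueprint with Suppressor, Magazine and Stock parts, each matched to a family of attachment item classes.
; GetStaticMeshComponent checks a given item class against the suppressor, magazine and stock variants in sequence and returns the matching component.
; Matching uses hardcoded class comparisons, and the construction script is empty.
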(fn ConstructionScript)

(fn GetStaticMeshComponent
  (params (ItemClass :type BP%20Item%20Class%20Reference))
  (Utilities|FlowControl|Sequence
    (:then_0
      (if (or (== ItemClass "/Game/Gun/BluePrints/BP_Suppressor1.BP_Suppressor1_C") (== ItemClass "/Game/Gun/BluePrints/BP_Suppressor2.BP_Suppressor2_C"))
        (return (Variables|Default|GetSuppressor))))
    (:then_1
      (if (Math|Boolean|ORBoolean (== ItemClass "/Game/Gun/BluePrints/BP_Magazine1.BP_Magazine1_C") (== ItemClass "/Game/Gun/BluePrints/BP_Magazine2.BP_Magazine2_C") (== ItemClass "/Game/Gun/BluePrints/BP_Magazine3.BP_Magazine3_C"))
        (return (Variables|Default|GetMagazine))))
    (:then_2
      (if (Math|Boolean|ORBoolean (== ItemClass "/Game/Gun/BluePrints/BP_Stock1.BP_Stock1_C") (== ItemClass "/Game/Gun/BluePrints/BP_Stock2.BP_Stock2_C") (== ItemClass "/Game/Gun/BluePrints/BP_Stock3.BP_Stock3_C"))
        (return (Variables|Default|GetStock))))))