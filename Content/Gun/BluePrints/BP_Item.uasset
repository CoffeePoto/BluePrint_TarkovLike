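; BP_Item is a world pickup actor that hands its ItemObject to the player's inventory on overlap.
; On BeginPlay it fills an invalid ItemObject from GetDefaultItemObject, which returns nothing here and appears intended for child Blueprints to override.
; When a BP_ThirdPersonCharacter enters the Box, it calls TryAddItem on that character's inventory component and destroys itself only if the add succeeds.
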(event OnComponentBeginOverlap(Box)
  (params (OverlappedComponent :type Primitive%20Component%20Object%20Reference) (OtherActor :type Actor%20Object%20Reference) (OtherComp :type Primitive%20Component%20Object%20Reference) (OtherBodyIndex :type Integer) (bFromSweep :type Boolean) (SweepResult :type Hit%20Result%20Structure%20%28by%20ref%29))
  (bind _asbp_third_person_character (Utilities|Casting|CastToBP_ThirdPersonCharacter OtherActor))
  (bind _added (Default|TryAddItem (Variables|/Game/ThirdPerson/Blueprints/BP_ThirdPersonCharacter.BP_ThirdPersonCharacter_C|GetAC_InventoryComponent _asbp_third_person_character) (Variables|Private|GetItemObject)))
  (if _added
    (Actor|DestroyActor)))

(event EventBeginPlay
  (if (not (Utilities|IsValid (Variables|Private|GetItemObject)))
    (bind _itemobject (Private|GetDefaultItemObject))
    (Variables|Private|SetItemObject _itemobject)))

(fn ConstructionScript)

(fn GetDefaultItemObject
  (return 0))