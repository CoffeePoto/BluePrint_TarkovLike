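; AI controller for ZMIKE characters that hands their behavior to the BT_ZMIKE behavior tree.
; On possession, it initializes the BB_ZMIKE blackboard with a patrol wait time and the pawn's current location as its original location.
; It then starts the tree, with no further decision logic in the controller itself.
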(event EventPossess
  (params (PossessedPawn :type Pawn%20Object%20Reference))
  (Utilities|FlowControl|Sequence
    (:then_0
      (Class|AIController|UseBlackboard "/Game/RadicalMike/BluePrints/AI/BB_ZMIKE.BB_ZMIKE")
      (AI|Components|Blackboard|SetValueasFloat (Variables|Default|GetBlackboard) (Variables|Default|GetPatrolWaitTimeKey) (Variables|Default|GetPatrolWaitTime))
      (AI|Components|Blackboard|SetValueasVector (Variables|Default|GetBlackboard) (Variables|Default|GetOriginalLocationKey) (Transformation|GetActorLocation PossessedPawn)))
    (:then_1
      (AI|RunBehaviorTree "/Game/RadicalMike/BluePrints/AI/BT_ZMIKE.BT_ZMIKE"))))

(fn ConstructionScript)