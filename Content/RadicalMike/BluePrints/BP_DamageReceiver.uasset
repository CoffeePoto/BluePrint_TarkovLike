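; BP_DamageReceiver tracks hit points and handles incoming damage, starting at MaxHP on BeginPlay.
; Each accepted hit subtracts damage and opens a timed invulnerability window, during which further damage is ignored until a timer restores vulnerability.
; It broadcasts current and max HP after every accepted hit, first clamping HP at zero and signalling death when health runs out.
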(event Custom|OnDamagedReceived
  (params (Damage :type Float%20%28double-precision%29))
  (if (Variables|Default|GetVulnerable)
    (Variables|Default|SetVulnerable false)
    (Utilities|Time|SetTimerbyEvent (delegate Custom|ReturnToVulnerable) (Variables|Default|GetInvulnerableTime))
    (Variables|Default|SetCurrentHP (- (Variables|Default|GetCurrentHP) Damage))
    (if (<= (Variables|Default|GetCurrentHP) 0.0)
      (Variables|Default|SetCurrentHP 0.0)
      (Default|CallOnDead)
      (Default|CallOnHealthPowerChanged (Variables|Default|GetCurrentHP) (Variables|Default|GetMaxHP))
      (else
        (Default|CallOnHealthPowerChanged (Variables|Default|GetCurrentHP) (Variables|Default|GetMaxHP))))))

(event Custom|ReturnToVulnerable
  (Variables|Default|SetVulnerable true))

(event EventBeginPlay
  (Variables|Default|SetCurrentHP (Variables|Default|GetMaxHP)))