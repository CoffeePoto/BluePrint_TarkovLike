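; BP_ZMIKE is an AI enemy character that senses, chases and attacks BP_ThirdPersonCharacter.
; SetState mirrors its state enum to the Blackboard and plays that state's montage.
; PawnSensing sets the target, with a one-time gun-load before chasing, while Tick returns it to Idle on lost range or target state.
; BPDamageReceiver handles damage and death; hit reactions resume chase or attack montages, and death disables collision before delayed destruction.
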(event OnSeePawn(PawnSensing)
  (params (Pawn :type Pawn%20Object%20Reference))
  (switch Utilities|FlowControl|Switch|SwitchonEMonsterState (Variables|Default|GetStateBP)
    (:NewEnumerator0
      _)
    (:NewEnumerator5
      _))
  (bind _asbp_third_person_character (Utilities|Casting|CastToBP_ThirdPersonCharacter Pawn))
  (if (Utilities|Enum|NotEqual(Enum) (Variables|/Game/ThirdPerson/Blueprints/BP_ThirdPersonCharacter.BP_ThirdPersonCharacter_C|GetStateBP _asbp_third_person_character) "NewEnumerator3")
    (AI|Components|Blackboard|SetValueasObject (Variables|/Script/AIModule.AIController|GetBlackboard (AI|GetAIController self)) (Variables|Default|GetTargetPlayerKey) Pawn)
    (if (Variables|Default|GetFirstEnter)
      (CallFunction|SetState "NewEnumerator5")
      (Variables|Default|SetFirstEnter false)
      (Utilities|FlowControl|Delay 3.0)
      (else
        (CallFunction|SetState "NewEnumerator2")))))

(event Custom|SetState
  (params (NewState :type EMonsterState%20Enum :default "NewEnumerator0"))
  (if (Utilities|Enum|NotEqual(Enum) (Variables|Default|GetStateBP) NewState)
    (AI|Components|Blackboard|SetValueasEnum (Variables|/Script/AIModule.AIController|GetBlackboard (AI|GetAIController self)) (Variables|Default|GetStateKey) NewState)
    (bind _output_get (Variables|Default|SetStateBP NewState))
    (switch Utilities|FlowControl|Switch|SwitchonEMonsterState _output_get
      (:NewEnumerator5
        (CallFunction|LoadGun))
      (:NewEnumerator2
        (CallFunction|PlayChase))
      (:NewEnumerator3
        (CallFunction|FireStart))
      (:NewEnumerator4
        (CallFunction|OnDead)))))

(event Custom|ZMIKE_Dead
  (Collision|SetCollisionEnabled (Variables|Collision|GetCapsuleComponent) "NoCollision")
  (CallFunction|SetState "NewEnumerator4")
  (Utilities|FlowControl|Delay 3.0)
  (Actor|DestroyActor))

(event Custom|TurnToTarget
  (params (Target :type Actor%20Object%20Reference))
  (Transformation|SetActorRotation (Math|Rotator|MakeRotator 0.0 0.0 (.yaw (Math|Rotator|MakeRotfromX (- (Transformation|GetActorLocation Target) (Transformation|GetActorLocation)))))))

(event Custom|LoadGun
  (Animation|PlayAnimMontage "/Game/RadicalMike/Animations/AM_LoadGun.AM_LoadGun" 1.0 "aggro"))

(event Custom|FireStart
  (Animation|PlayAnimMontage "/Game/RadicalMike/Animations/AM_Attack.AM_Attack" 1.0 "FireStart"))

(event Custom|OnDead
  (Animation|Montage|PlayMontage (Variables|Character|GetMesh) "/Game/RadicalMike/Animations/AM_Dead.AM_Dead" 1.0 0.0 "Dead"))

(event Custom|PlayChase
  (Animation|Montage|PlayMontage 0 "/Game/RadicalMike/Animations/AM_Chase.AM_Chase" 1.0 0.0 "Chase"))

(event EventBeginPlay
  (EventDispatchers|BindEventtoOnDead (Variables|Default|GetBP_DamageReceiver) (delegate Custom|ZMIKE_Dead)))

(event Game|Damage|EventAnyDamage
  (params (Damage :type Float%20%28single-precision%29) (DamageType :type Damage%20Type%20Object%20Reference) (InstigatedBy :type Controller%20Object%20Reference) (DamageCauser :type Actor%20Object%20Reference))
  (Default|OnDamagedReceived (Variables|Default|GetBP_DamageReceiver) Damage)
  (if (Utilities|Enum|NotEqual(Enum) (Variables|Default|GetStateBP) "NewEnumerator4")
    (Animation|Montage|PlayMontage (Variables|Character|GetMesh) "/Game/RadicalMike/Animations/AM_Hit.AM_Hit" 1.0 0.0 "Front"
      (:OnCompleted
        (switch Utilities|FlowControl|Switch|SwitchonEMonsterState (Variables|Default|GetStateBP)
          (:NewEnumerator2
            (CallFunction|PlayChase))
          (:NewEnumerator3
            (CallFunction|FireStart)))))))

(event EventTick
  (params (DeltaSeconds :type Float%20%28single-precision%29))
  (switch Utilities|FlowControl|Switch|SwitchonEMonsterState (Variables|Default|GetStateBP)
    (:NewEnumerator2
      (CallFunction|OnChase))
    (:NewEnumerator3
      (CallFunction|OnAttack))
    (:NewEnumerator4
      (CallFunction|ZMIKEDead))))

(fn ConstructionScript)

(fn OnChase
  (bind _as액터 (Utilities|Casting|CastToActor (AI|Components|Blackboard|GetValueasObject (AI|GetBlackboard (AI|GetAIController self)) (Variables|Default|GetTargetPlayerKey))))
  (if (> (Transformation|GetDistanceTo _as액터) (Variables|/Script/AIModule.PawnSensingComponent|GetSightRadius (Variables|Default|GetPawnSensing)))
    (CallFunction|SetState "NewEnumerator0")))

(fn OnAttack
  (bind _asbp_third_person_character (Utilities|Casting|CastToBP_ThirdPersonCharacter (AI|Components|Blackboard|GetValueasObject (AI|GetBlackboard (AI|GetAIController self)) (Variables|Default|GetTargetPlayerKey))))
  (if (Utilities|Enum|Equal(Enum) (Variables|/Game/ThirdPerson/Blueprints/BP_ThirdPersonCharacter.BP_ThirdPersonCharacter_C|GetStateBP _asbp_third_person_character) "NewEnumerator3")
    (CallFunction|SetState "NewEnumerator0")))